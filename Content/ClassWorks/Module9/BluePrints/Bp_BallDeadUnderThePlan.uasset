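; Functional test that checks the playing ball dies only after passing below the pawn's paddle cube along the X axis.
; PrepareTest caches the player pawn's Cube world location and binds to its PlayingBall's OnDead event.
; On death, the test succeeds if the ball sphere's X is less than the cached cube X, otherwise it fails.
; StartTest and Tick are unused.
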(event Custom|OnDead_Event_0
  (if (< (.x (Transformation|GetWorldLocation (Variables|/Game/HomeWorks/HomeWork6(9_3)/BluePrints/Actors/Bp_ActorCollision.Bp_ActorCollision_C|GetSphere (Variables|Default|GetBall)))) (.x (Variables|Default|GetPawn%20Location)))
    (Class|FunctionalTest|FinishTest "Succeeded")
    (else
      (Class|FunctionalTest|FinishTest "Failed"))))

(event EventPrepareTest
  (bind _asbp_pawn (Utilities|Casting|CastToBp_Pawn (Game|Player|GetPlayerPawn 0)))
  (Variables|Default|SetPawn%20Location (Transformation|GetWorldLocation (Variables|/Game/HomeWorks/HomeWork6(9_3)/BluePrints/Pawns/Bp_Pawn.Bp_Pawn_C|GetCube _asbp_pawn)))
  (bind _output_get (Variables|Default|SetBall (Variables|/Game/HomeWorks/HomeWork6(9_3)/BluePrints/Pawns/Bp_Pawn.Bp_Pawn_C|GetPlayingBall _asbp_pawn)))
  (EventDispatchers|AssignOnDead _output_get (delegate Custom|OnDead_Event_0)))

(event EventStartTest)

(event EventTick
  (params (DeltaSeconds :type Float%20%28single-precision%29)))

(fn ConstructionScript)