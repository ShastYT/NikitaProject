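; Homework block actor that shrinks each time another actor begins overlapping it.
; On BeginPlay it stores five percent of its starting scale, then subtracts that fixed step from its current scale on every overlap, so shrinking is linear.
; The overlapping actor is not filtered, and the graph has no lower limit or destroy step despite the "Des" in the asset name.
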(event EventBeginPlay
  (|CallParentFunction)
  (Variables|Default|Set5precent (* (Transformation|GetActorScale3D) 0.05)))

(event Collision|EventActorBeginOverlap
  (params (OtherActor :type Actor%20Object%20Reference))
  (|CallParentFunction OtherActor)
  (Transformation|SetActorScale3D (- (Transformation|GetActorScale3D) (Variables|Default|Get5precent))))

(event EventTick
  (params (DeltaSeconds :type Float%20%28single-precision%29))
  (|CallParentFunction DeltaSeconds) ; This node is disabled and will not be called.\nDrag off pins to build functionality.
)

(fn ConstructionScript
  (|CallParentFunction))