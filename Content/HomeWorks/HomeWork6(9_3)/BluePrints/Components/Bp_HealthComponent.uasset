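; Health component that tracks an owner's hit points and signals health changes and death through event dispatchers.
; Add and Sub change Hp by one through Update, with no clamping.
; Update fires OnHealthUpdate before storing the new Hp, then fires OnDeath when IsDead finds Hp at or below zero.
; The event graph holds only disabled BeginPlay and Tick stubs.
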(event EventBeginPlay)

(event EventTick
  (params (DeltaSeconds :type Float%20%28single-precision%29)))

(fn Update
  (params (Hp :type Integer))
  (Default|CallOnHealthUpdate)
  (Variables|Default|SetHp Hp)
  (if (CallFunction|IsDead)
    (Default|CallOnDeath)))

(fn Sub
  (CallFunction|Update (- (Variables|Default|GetHp) 1)))

(fn Add
  (CallFunction|Update (+ (Variables|Default|GetHp) 1)))

(fn IsDead
  (return (<= (Variables|Default|GetHp) 0)))