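; Speed component that computes speed changes and broadcasts them through an OnSpeedUpdate event dispatcher.
; Mult and Divide scale the passed-in speed up or down by fixed factors, while Reset restores SpeedPrec to its default.
; All three route through Update, which sends SpeedPrec as the old value and the result as the new one, without storing the result.
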(event EventBeginPlay)

(event EventTick
  (params (DeltaSeconds :type Float%20%28single-precision%29)))

(fn Mult
  (params (OldSpeed :type Float%20%28single-precision%29))
  (CallFunction|Update (* OldSpeed 1.3)))

(fn Divide
  (params (OldSpeed :type Float%20%28single-precision%29))
  (CallFunction|Update (* OldSpeed 0.7)))

(fn Update
  (params (Speed :type Float%20%28single-precision%29))
  (Default|CallOnSpeedUpdate (Variables|Default|GetSpeedPrec) Speed))

(fn Reset
  (bind _output_get (Variables|Default|SetSpeedPrec 1.0))
  (CallFunction|Update _output_get))