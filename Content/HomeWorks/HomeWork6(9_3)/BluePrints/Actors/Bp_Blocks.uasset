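; Bp_Blocks is a breakable block actor that starts with three HP and loses health when hit by Bp_ActorCollision.
; Its health component exposes update and death events, bound on BeginPlay, alongside functions that swap the cube's material or spawn Bp_Bonus and destroy the block.
; BeginPlay also spawns an X-by-Y grid of Bp_Blocks at padded world-origin positions, so the class spawns itself and each copy runs the same logic.
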(event EventBeginPlay
  (bind _padding (Variables|Default|GetPadding))
  (Variables|/Game/HomeWorks/HomeWork6(9_3)/BluePrints/Components/Bp_HealthComponent.Bp_HealthComponent_C|SetHp (Variables|Default|GetBp_HealthComponent) 3)
  (CallFunction|Binds)
  (for _index (range 0 (Variables|Default|GetX))
    (for _index_2 (range 0 (Variables|Default|GetY))
      (Game|SpawnActorfromClass "Bp_Blocks_C" (Math|Transform|MakeTransform (Math|Vector|MakeVector (Math|Conversions|ToFloat(Integer) (* _index _padding)) (Math|Conversions|ToFloat(Integer) (* _index_2 _padding)) 0.0)) "Undefined" 0 0))))

(event Collision|EventActorBeginOverlap
  (params (OtherActor :type Actor%20Object%20Reference)))

(event EventTick
  (params (DeltaSeconds :type Float%20%28single-precision%29)))

(event Collision|EventHit
  (params (MyComp :type Primitive%20Component%20Object%20Reference) (Other :type Actor%20Object%20Reference) (OtherComp :type Primitive%20Component%20Object%20Reference) (bSelfMoved :type Boolean) (HitLocation :type Vector :default "0, 0, 0") (HitNormal :type Vector :default "0, 0, 0") (NormalImpulse :type Vector :default "0, 0, 0") (Hit :type Hit%20Result%20Structure%20%28by%20ref%29))
  (Utilities|Casting|CastToBp_ActorCollision Other)
  (Default|Sub (Variables|Default|GetBp_HealthComponent)))

(fn ConstructionScript)

(fn Binds
  (bind _bp_healthcomponent (Variables|Default|GetBp_HealthComponent))
  (EventDispatchers|BindEventtoOnHealthUpdate _bp_healthcomponent (EventDispatchers|CreateEvent :!event SetMaterial))
  (EventDispatchers|BindEventtoOnDeath _bp_healthcomponent (EventDispatchers|CreateEvent :!event SpawnBonus)))

(fn SetMaterial
  (Rendering|Material|SetMaterial (Variables|Default|GetCube) 0 "/Engine/Functions/Engine_MaterialFunctions02/ExampleContent/GradientMap_Multi_Example.GradientMap_Multi_Example"))

(fn SpawnBonus
  (Game|SpawnActorfromClass "/Game/HomeWorks/HomeWork6(9_3)/BluePrints/Actors/Bp_Bonus.Bp_Bonus_C" (Transformation|GetActorTransform) "Undefined" 0 0)
  (Actor|DestroyActor))