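; Bp_Bonus is a moving bonus pickup actor that reacts when a Bp_Pawn overlaps it.
; On BeginPlay it randomly flags itself as a ball or weight bonus and sets the sphere material to match.
; Tick moves it with a swept offset along Direction at Speed.
; On overlap, ApplyBonus widens the bonus actor's own X scale, without reading the type flags or affecting the pawn.
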(event EventBeginPlay
  (CallFunction|GetBonusType))

(event Collision|EventActorBeginOverlap
  (params (OtherActor :type Actor%20Object%20Reference))
  (Utilities|Casting|CastToBp_Pawn OtherActor)
  (CallFunction|ApplyBonus))

(event EventTick
  (params (DeltaSeconds :type Float%20%28single-precision%29))
  (Transformation|AddActorWorldOffset (* (* (Variables|Default|GetDirection) (Variables|Default|GetSpeed)) DeltaSeconds) true))

(fn ConstructionScript)

(fn ApplyBonus
  (bind _returnvalue (Transformation|GetActorScale3D))
  (Transformation|SetActorScale3D (Math|Vector|MakeVector (+ (.x _returnvalue) 5.0) (.y _returnvalue) (.z _returnvalue))))

(fn GetBonusType
  (bind _sphere (Variables|Default|GetSphere))
  (if (Math|Random|RandomBool)
    (Variables|Default|SetBonusBall true)
    (Rendering|Material|SetMaterial _sphere 0 "/Game/Default/FirstPerson/Meshes/FirstPersonProjectileMaterial.FirstPersonProjectileMaterial")
    (else
      (Variables|Default|SetBonusWeight true)
      (Rendering|Material|SetMaterial _sphere 0 "/Game/Default/StarterContent/Materials/M_Basic_Floor.M_Basic_Floor"))))