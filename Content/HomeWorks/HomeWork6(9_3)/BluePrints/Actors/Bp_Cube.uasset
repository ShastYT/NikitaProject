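; Breakable cube actor that loses health when hit by a Bp_ActorCollision and may drop a bonus when destroyed.
; On BeginPlay it binds to its health component's events and randomly becomes either a tougher bonus cube or a one-hit plain cube.
; Health updates swap the mesh material to match remaining HP.
; On death, bonus cubes spawn a random size, speed or ball pickup before the actor destroys itself.
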(event EventBeginPlay
  (CallFunction|Binds)
  (CallFunction|GetBonusStatus))

(event Collision|EventActorBeginOverlap
  (params (OtherActor :type Actor%20Object%20Reference)))

(event EventTick
  (params (DeltaSeconds :type Float%20%28single-precision%29)))

(event Collision|EventHit
  (params (MyComp :type Primitive%20Component%20Object%20Reference) (Other :type Actor%20Object%20Reference) (OtherComp :type Primitive%20Component%20Object%20Reference) (bSelfMoved :type Boolean) (HitLocation :type Vector :default "0, 0, 0") (HitNormal :type Vector :default "0, 0, 0") (NormalImpulse :type Vector :default "0, 0, 0") (Hit :type Hit%20Result%20Structure%20%28by%20ref%29))
  (Utilities|Casting|CastToBp_ActorCollision Other)
  (Default|Sub (Variables|Default|GetBp_HealthComponent)))

(fn ConstructionScript)

(fn Binds
  (bind _bp_healthcomponent (Variables|Default|GetBp_HealthComponent))
  (EventDispatchers|BindEventtoOnHealthUpdate _bp_healthcomponent (EventDispatchers|CreateEvent :!event SetMaterial))
  (EventDispatchers|BindEventtoOnDeath _bp_healthcomponent (EventDispatchers|CreateEvent :!event SpawnBonus)))

(fn SetMaterial
  (params (OldHealth :type Integer) (NewHealth :type Integer))
  (Rendering|Material|SetMaterial (Variables|Default|GetStaticMesh) 0 (Utilities|Array|Get(acopy) (Utilities|Array|MakeArray "/Game/Default/Geometry/Meshes/CubeMaterial.CubeMaterial" "/Game/Default/StarterContent/Materials/M_Metal_Copper.M_Metal_Copper" "/Game/Default/StarterContent/Materials/M_Metal_Gold.M_Metal_Gold") (- (Variables|/Game/HomeWorks/HomeWork6(9_3)/BluePrints/Components/Bp_HealthComponent.Bp_HealthComponent_C|GetHp (Variables|Default|GetBp_HealthComponent)) 1))))

(fn SpawnBonus
  (if (Variables|Default|GetIsBonus)
    (Game|SpawnActorfromClass (Utilities|Array|Get(acopy) (Utilities|Array|MakeArray "/Game/HomeWorks/HomeWork6(9_3)/BluePrints/Actors/Bp_BonusSize.Bp_BonusSize_C" "/Game/HomeWorks/HomeWork6(9_3)/BluePrints/Actors/Bp_BonusSpeed.Bp_BonusSpeed_C" "/Game/HomeWorks/HomeWork6(9_3)/BluePrints/Actors/Bp_BonusBall.Bp_BonusBall_C") (Math|Random|RandomIntegerinRange 0 2)) (Transformation|GetActorTransform) "Undefined" 0 0))
  (Actor|DestroyActor))

(fn GetBonusStatus
  (bind _bp_healthcomponent (Variables|Default|GetBp_HealthComponent))
  (bind _output_get (Variables|Default|SetIsBonus (Math|Random|RandomBoolwithWeight 0.25)))
  (if _output_get
    (Variables|/Game/HomeWorks/HomeWork6(9_3)/BluePrints/Components/Bp_HealthComponent.Bp_HealthComponent_C|SetHp _bp_healthcomponent 3)
    (else
      (Variables|/Game/HomeWorks/HomeWork6(9_3)/BluePrints/Components/Bp_HealthComponent.Bp_HealthComponent_C|SetHp _bp_healthcomponent 1))))