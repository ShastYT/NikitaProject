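; Bp_FlipFlopLamp is a lamp actor whose point light blinks a limited number of times after play begins.
; After an initial delay, BeginPlay enters a DoN loop capped by LightFlipCount.
; Each pass toggles the light's visibility twice through LightVisibility, waiting LightToggleSpeed after each toggle, then loops back without using Tick.
; The DoN is never reset, so blinking stops once the count runs out.
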(event EventBeginPlay
  (Utilities|FlowControl|Delay (Variables|Default|GetDelay))
  (Utilities|FlowControl|DoN (Variables|Default|GetLightFlipCount) :!label _label
    (:Exit
      (CallFunction|LightVisibility)
      (Utilities|FlowControl|Delay (Variables|Default|GetLightToggleSpeed))
      (CallFunction|LightVisibility)
      (Utilities|FlowControl|Delay (Variables|Default|GetLightToggleSpeed))
      (goto _label))))

(event Collision|EventActorBeginOverlap
  (params (OtherActor :type Actor%20Object%20Reference)))

(event EventTick
  (params (DeltaSeconds :type Float%20%28single-precision%29)))

(fn ConstructionScript)

(fn LightVisibility
  (Rendering|ToggleVisibility (Variables|Default|GetPointLight) false))