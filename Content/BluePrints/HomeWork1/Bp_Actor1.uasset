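; Bp_Actor1 is an actor that spins one of two cube components at a time, alternating between them.
; On BeginPlay, a FlipFlop followed by a one-second Delay loops back on itself, toggling the RotateFirstCube flag each second.
; Tick reads that flag and calls CubeRotation or Cube1Rotation, each adding a fixed per-frame world rotation on a different axis, so spin speed depends on frame rate.
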(event EventBeginPlay
  (Utilities|FlowControl|FlipFlop :!label _label
    (:A
      (Variables|Default|SetRotateFirstCube false))
    (:B
      (Variables|Default|SetRotateFirstCube true)))
  (Utilities|FlowControl|Delay 1.0)
  (goto _label))

(event Collision|EventActorBeginOverlap
  (params (OtherActor :type Actor%20Object%20Reference)))

(event EventTick
  (params (DeltaSeconds :type Float%20%28single-precision%29))
  (if (Variables|Default|GetRotateFirstCube)
    (CallFunction|CubeRotation)
    (else
      (CallFunction|Cube1Rotation))))

(fn ConstructionScript)

(fn CubeRotation
  (Transformation|AddWorldRotation (Variables|Default|GetCube) "0, 0,15.000000" false false))

(fn Cube1Rotation
  (Transformation|AddWorldRotation (Variables|Default|GetCube1) "15.000000, 0, 0" false false))